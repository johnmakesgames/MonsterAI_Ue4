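; Base weapon Blueprint that child weapons extend, handling firing, ammo, sound, muzzle FX and equip animations for the player.
; Fire checks the player character's pool for the AmmoType (melee is free), plays sound through SoundManager, deducts cost with a HUD update, then starts the FPS arms animation.
; Infinite firing skips ammo checks and cost.
; LaunchProjectile, triggered by anim notify, spawns the projectile at a muzzle socket; LaunchMelee is an empty stub.
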(fn `CheckAmmo`
  (returns (DoesHaveEnoughAmmo :type Boolean))
  ;[1 1 1] Depending on ammo type, check the current ammo amount against the shot cost and if it's greater or equal to zero we can fire. Limited to Mana only
  (switch `/Game/Blueprints/Weapons/AmmoTypes` (`self.AmmoType`)
    (:`NewEnumerator0`
      (return (>= (- (`/Game/Blueprints/BasePlayerCharacter.Mana` (cast `/Game/Blueprints/BasePlayerCharacter` (`GameplayStatics.GetPlayerCharacter` 0) :!pure true)) (`self.ShotCost`)) 0)))
    (:`NewEnumerator1`
      (return (>= (- (`/Game/Blueprints/BasePlayerCharacter.Bullets` (cast `/Game/Blueprints/BasePlayerCharacter` (`GameplayStatics.GetPlayerCharacter` 0) :!pure true)) (`self.ShotCost`)) 0)))
    (:`NewEnumerator2`
      (return (>= (- (`/Game/Blueprints/BasePlayerCharacter.Missile` (cast `/Game/Blueprints/BasePlayerCharacter` (`GameplayStatics.GetPlayerCharacter` 0) :!pure true)) (`self.ShotCost`)) 0)))
    (:`NewEnumerator3`
      ;[1 1 1] Melee Always has enough ammo, no stamina system..
      (return true))))

(fn `ConsumeAmmo`
  ;[1 1 1] Consume Ammo, currently limited to Mana only
  (switch `/Game/Blueprints/Weapons/AmmoTypes` (`self.AmmoType`)
    (:`NewEnumerator0`
      (`self.DeductMana`))
    (:`NewEnumerator1`
      (`self.DeductBullets`))
    (:`NewEnumerator2`
      (`self.DeductMissiles`))
    (:`NewEnumerator3`
      (return)))
  (return))

(fn `DeductBullets`
  (bind _asbase_player_character (cast `/Game/Blueprints/BasePlayerCharacter` (`GameplayStatics.GetPlayerCharacter` 0) :!pure true))
  (bind _output_get (set `/Game/Blueprints/BasePlayerCharacter.Bullets` (- (`/Game/Blueprints/BasePlayerCharacter.Bullets` _asbase_player_character) (`self.ShotCost`)) _asbase_player_character))
  (`/Game/Blueprints/UI/InGameHud.SetAmmo` (`/Game/Blueprints/BasePlayerController.UIReference` (cast `/Game/Blueprints/BasePlayerController` (`GameplayStatics.GetPlayerController` 0) :!pure true)) (`KismetTextLibrary.Conv_IntToText` _output_get) "/Game/Effects/FX_UsedByGregAndAde/BulletPickupGraphic.BulletPickupGraphic")
  (return))

(fn `DeductMana`
  (bind _asbase_player_character (cast `/Game/Blueprints/BasePlayerCharacter` (`GameplayStatics.GetPlayerCharacter` 0) :!pure true))
  (bind _output_get (set `/Game/Blueprints/BasePlayerCharacter.Mana` (- (`/Game/Blueprints/BasePlayerCharacter.Mana` _asbase_player_character) (`self.ShotCost`)) _asbase_player_character))
  (`/Game/Blueprints/UI/InGameHud.SetAmmo` (`/Game/Blueprints/BasePlayerController.UIReference` (cast `/Game/Blueprints/BasePlayerController` (`GameplayStatics.GetPlayerController` 0) :!pure true)) (`KismetTextLibrary.Conv_IntToText` _output_get) "/Game/Effects/FX_UsedByGregAndAde/ManaPickupGraphic.ManaPickupGraphic")
  (return))

(fn `DeductMissiles`
  (bind _asbase_player_character (cast `/Game/Blueprints/BasePlayerCharacter` (`GameplayStatics.GetPlayerCharacter` 0) :!pure true))
  (bind _output_get (set `/Game/Blueprints/BasePlayerCharacter.Missile` (- (`/Game/Blueprints/BasePlayerCharacter.Missile` _asbase_player_character) (`self.ShotCost`)) _asbase_player_character))
  (`/Game/Blueprints/UI/InGameHud.SetAmmo` (`/Game/Blueprints/BasePlayerController.UIReference` (cast `/Game/Blueprints/BasePlayerController` (`GameplayStatics.GetPlayerController` 0) :!pure true)) (`KismetTextLibrary.Conv_IntToText` _output_get) "/Game/Effects/FX_UsedByGregAndAde/MissileGraphicPickup.MissileGraphicPickup")
  (return))

(fn `Equip`
  ;[1 1 1] Play an animation, this needs reworking for each child class as animations will be different and cannot be variables
  (`SkeletalMeshComponent.PlayAnimation` (`self.WeaponMesh`) null false)
  (return))

(fn `Fire`
  (set `self.isFiring` true)
  (bind _doeshaveenoughammo (`self.CheckAmmo`))
  (if (or _doeshaveenoughammo (`self.isinfinitefiring`))
    (`self.PlayFireSound`)
    (if (`self.isinfinitefiring`)
      (`self.PlayFireAnimation`)
      (return)
      (else
        (`self.ConsumeAmmo`)
        (`self.PlayFireAnimation`)
        (return)))
    (else
      (set `self.isFiring` false)
      (return))))

(fn `FiringDelay`
  ;[1 1 1] Boolean that is toggled via a timer set in the fire function.
  (set `self.canFire` true)
  (return))

(fn `Init`
  (params (InventoryReferenec :type "/Game/Blueprints/Inventory Object Reference"))
  ;[1 1 1] On Spawn store a referenec to the inventory, this allows to get the players ammo
  (set `self.InventoryReference` InventoryReferenec)
  (bind _outactors (`GameplayStatics.GetAllActorsOfClass` "/Game/Blueprints/SoundManager.SoundManager_C"))
  (set `self.SoundManager` (`|GetArrayItem` _outactors))
  (return))

(fn `LaunchMelee`
  ;[1 1 1] This is triggered by  an anim notify
  (return))

(fn `LaunchProjectile`
  ;[1 1 1] This is triggered by  an anim notify
  (`|SpawnActorFromClass` (`self.ProjectileType`) (`SceneComponent.GetSocketTransform` (`self.WeaponMesh`) (`self.ProjectileSpawnSocketName`) "RTS_World") "AlwaysSpawn" "OverrideRootScale" null (cast `/Game/Blueprints/BasePlayerCharacter` (`self.GetOwner` (`self.InventoryReference`)) :!pure true))
  (return))

(fn `PlayEquipAnimation`
  ;[1 1 1] Such finished much blueprint
  (return))

(fn `PlayFireAnimation`
  (bind _asfpsarm_blueprint (cast `/Game/Blueprints/FPSArmBlueprint` (`SkeletalMeshComponent.GetAnimInstance` (`/Game/Blueprints/BasePlayerCharacter.FpsArms` (cast `/Game/Blueprints/BasePlayerCharacter` (`GameplayStatics.GetPlayerPawn` 0) :!pure true))) :!pure true))
  ;[1 1 1] Such finished much blueprint
  (`/Game/Blueprints/FPSArmBlueprint.StartFiring` _asfpsarm_blueprint)
  (set `/Game/Blueprints/FPSArmBlueprint.FirePlayRate` (`self.FireSpeed`) _asfpsarm_blueprint)
  (return))

(fn `PlayFireSound`
  (bind _soundmanager (`self.SoundManager`))
  ;[1 1 1] Play a fire sound at a muzzle socket, defined by designer
  (`/Engine/EditorBlueprintResources/StandardMacros.IsValid` _soundmanager
    (:`Is Valid`
      (`/Game/Blueprints/SoundManager.PlaySFX` _soundmanager (`self.FireSound`) (`SceneComponent.GetSocketLocation` (`self.WeaponMesh`) (`self.ProjectileSpawnSocketName`)))
      (return))
    (:`Is Not Valid`
      (bind _outactors (`GameplayStatics.GetAllActorsOfClass` "/Game/Blueprints/SoundManager.SoundManager_C"))
      (bind _output_get (set `self.SoundManager` (`|GetArrayItem` _outactors)))
      (`/Game/Blueprints/SoundManager.PlaySFX` _output_get (`self.FireSound`) (0.0 0.0 0.0))
      (return))))

(fn `PlayMuzzleFX`
  ;[1 1 1] Spawn Muzzle FX, only needed for range weapons.
  (`GameplayStatics.SpawnEmitterAtLocation` (`self.MuzzleEmitter`) (`SceneComponent.GetSocketLocation` (`self.WeaponMesh`) (`self.ProjectileSpawnSocketName`)))
  (return))

(fn `PlayPutAwayAnimation`
  ;[1 1 1] Such finished much blueprint
  (return))

(fn `PutAway`
  (set `self.canFire` false)
  (`SkeletalMeshComponent.PlayAnimation` (`self.WeaponMesh`) null false)
  (return))

(fn `UserConstructionScript`)