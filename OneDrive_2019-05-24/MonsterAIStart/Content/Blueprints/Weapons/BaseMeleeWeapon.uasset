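; Base melee weapon Blueprint that calculates attack damage from the player's stats.
; CalculateDamage adds the player's Strength to BaseDamage, then multiplies the sum by BerzerkDamage when that powerup value is above zero.
; It reads both stats by casting player 0 to BasePlayerCharacter rather than using the weapon's owner.
; The event graph is empty, and the construction script only calls its parent.
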(fn `CalculateDamage`
  (returns (Damage :type "Float (double-precision)"))
  (bind _berzerkdamage (`/Game/Blueprints/BasePlayerCharacter.BerzerkDamage` (cast `/Game/Blueprints/BasePlayerCharacter` (`GameplayStatics.GetPlayerPawn` 0) :!pure true)))
  (bind _returnvalue (+ (`self.BaseDamage`) (`KismetMathLibrary.Conv_IntToDouble` (`/Game/Blueprints/BasePlayerCharacter.Strength` (cast `/Game/Blueprints/BasePlayerCharacter` (`GameplayStatics.GetPlayerCharacter` 0) :!pure true)))))
  ;[1 1 1] Takes into account powerup Berzerk Damage if there is any, also applies strength as a modifier to weaken / strengthen attack
  (if (> _berzerkdamage 0.0)
    (return (* _berzerkdamage _returnvalue))
    (else
      (return _returnvalue))))

(fn `UserConstructionScript`
  (`parent.UserConstructionScript`))