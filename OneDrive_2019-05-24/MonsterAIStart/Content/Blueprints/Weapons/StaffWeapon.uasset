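; Staff weapon Blueprint that extends a parent weapon's fire logic to launch skull projectiles.
; On Fire it runs the parent logic, then, if IsFiring, spawns a SkullProjectile at the mesh's FirePoint socket, aimed along the player controller's control rotation.
; Each shot tints the staff mesh's GlowParameter blue, and a short timer resets it to white.
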(event `self.Fire`
  ;[1 1 1] Calls parent fire mechanic and spawns projectile
  (`parent.Fire`)
  (if (`self.isFiring`)
    (`|SpawnActorFromClass` "/Game/Blueprints/Weapons/Projectiles/SkullProjectile.SkullProjectile_C" (`KismetMathLibrary.MakeTransform` (`SceneComponent.GetSocketLocation` (`self.SK_Blunt_HellHammer_Cine`) "FirePoint") (`Controller.GetControlRotation` (`GameplayStatics.GetPlayerController` 0))) "Undefined" "OverrideRootScale" null null)
    (`MeshComponent.SetVectorParameterValueOnMaterials` (`self.SK_Blunt_HellHammer_Cine`) "GlowParameter" (0.0 4.0 12.0))
    (`KismetSystemLibrary.K2_SetTimerDelegate` (delegate `TurnOffGlow`) 0.75)))

(event `TurnOffGlow`
  (`MeshComponent.SetVectorParameterValueOnMaterials` (`self.SK_Blunt_HellHammer_Cine`) "GlowParameter" (1.0 1.0 1.0)))

(fn `UserConstructionScript`
  (`parent.UserConstructionScript`))