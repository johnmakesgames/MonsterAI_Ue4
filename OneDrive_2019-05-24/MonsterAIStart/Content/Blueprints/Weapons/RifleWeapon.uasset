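; Rifle weapon Blueprint that adds automatic projectile fire and camera shake on top of its parent weapon's behavior.
; Fire opens a Gate that loops through a short retriggerable delay, calling parent Fire and spawning a RifleProjectile at the Arrow's transform while IsFiring is true.
; StopFireAnim stops the weapon mesh and closes the Gate to end the loop.
; PlayFireAnimation extends the parent with a world camera shake centered on the player.
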(event `self.PlayFireAnimation`
  (`parent.PlayFireAnimation`)
  (`GameplayStatics.PlayWorldCameraShake` (`self.CameraShake`) (`self.K2_GetActorLocation` (`GameplayStatics.GetPlayerCharacter` 0)) 255.0 255.0))

(event `self.Fire`
  (bind _arrow (`self.Arrow`))
  ;[1 1 1] Calls parent fire mechanic and spawns projectile
  (`|ExecutionSequence`
    (:`then_0`
      (goto _label :!via `Open`))
    (:`then_1`
      (`/Engine/EditorBlueprintResources/StandardMacros.Gate` true :!label _label
        (:`Exit`
          (`|ExecutionSequence`
            (:`then_0`
              (`parent.Fire`)
              (if (`self.isFiring`)
                (`|SpawnActorFromClass` "/Game/Blueprints/Weapons/Projectiles/RifleProjectile.RifleProjectile_C" (`KismetMathLibrary.MakeTransform` (`SceneComponent.K2_GetComponentLocation` _arrow) (`SceneComponent.K2_GetComponentRotation` _arrow)) "AlwaysSpawn" "OverrideRootScale" null null)))
            (:`then_1`
              (`KismetSystemLibrary.RetriggerableDelay` 0.1)
              (goto _label))))))))

(event `/Game/Blueprints/Anims.StopFireAnim`
  ;[1 1 1] Calls parent fire mechanic and spawns projectile
  (`SkeletalMeshComponent.Stop` (`self.WeaponMesh`))
  (goto _label :!via `Close`))

(fn `UserConstructionScript`
  (`parent.UserConstructionScript`))