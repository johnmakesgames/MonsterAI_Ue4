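; Mana pickup that restores the player's mana, clamped to ManaMax, when a BasePlayerCharacter overlaps its collision.
; The amount comes from AmmoToGive and is applied to player pawn 0 rather than the overlapping actor.
; It asks its owning BasePickupFactory to respawn after the configured delay, plays sound and particles, then destroys itself.
; The HUD shows the new mana through the player controller's SetAmmo UI call.
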(event `self.PickupCollision.OnComponentBeginOverlap`
  (params (OverlappedComponent :type "PrimitiveComponent Object Reference") (OtherActor :type "Actor Object Reference") (OtherComp :type "PrimitiveComponent Object Reference") (OtherBodyIndex :type Integer) (bFromSweep :type Boolean) (SweepResult :type "HitResult Structure (by ref)"))
  (bind _asbase_pickup_factory (cast `/Game/Blueprints/Pickups/PickupFactories/BasePickupFactory` (`self.GetOwner`) :!pure true))
  (bind _asbase_player_character (cast `/Game/Blueprints/BasePlayerCharacter` (`GameplayStatics.GetPlayerPawn` 0) :!pure true))
  (bind (_pickupstructure_pickupclass _pickupstructure_respawndelay) (break `/Game/Blueprints/Pickups/PickupStructure` (`/Game/Blueprints/Pickups/PickupFactories/BasePickupFactory.PickupStructure` _asbase_pickup_factory)))
  (cast `/Game/Blueprints/BasePlayerCharacter` OtherActor)
  (bind _output_get (set `/Game/Blueprints/BasePlayerCharacter.Mana` (`KismetMathLibrary.Clamp` (+ (`/Game/Blueprints/BasePlayerCharacter.Mana` _asbase_player_character) (`self.AmmoToGive`)) 0 (`/Game/Blueprints/BasePlayerCharacter.ManaMax` _asbase_player_character)) _asbase_player_character))
  (`/Game/Blueprints/Pickups/PickupFactories/BasePickupFactory.ReSpawn` _asbase_pickup_factory _pickupstructure_respawndelay)
  (`self.PlaySound`)
  (`self.PlayParticles`)
  (`/Game/Blueprints/UI/InGameHud.SetAmmo` (`/Game/Blueprints/BasePlayerController.UIReference` (cast `/Game/Blueprints/BasePlayerController` (`GameplayStatics.GetPlayerController` 0) :!pure true)) (`KismetTextLibrary.Conv_IntToText` _output_get) null)
  (`self.K2_DestroyActor`))

(fn `UserConstructionScript`
  (`parent.UserConstructionScript`))