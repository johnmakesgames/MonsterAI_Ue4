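; Health pickup that heals a BasePlayerCharacter when it overlaps the pickup's collision.
; Below max health, it adds HealthToGive clamped to HealthMax, updates the health UI through player controller 0, plays sound and particles, then destroys itself.
; Before destruction it tells its owning BasePickupFactory to respawn after the delay in that factory's PickupStructure.
; At full health it only refreshes the UI and remains in the world.
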(event `self.PickupCollision.OnComponentBeginOverlap`
  (params (OverlappedComponent :type "PrimitiveComponent Object Reference") (OtherActor :type "Actor Object Reference") (OtherComp :type "PrimitiveComponent Object Reference") (OtherBodyIndex :type Integer) (bFromSweep :type Boolean) (SweepResult :type "HitResult Structure (by ref)"))
  (bind _asbase_pickup_factory (cast `/Game/Blueprints/Pickups/PickupFactories/BasePickupFactory` (`self.GetOwner`) :!pure true))
  (bind (_pickupstructure_pickupclass _pickupstructure_respawndelay) (break `/Game/Blueprints/Pickups/PickupStructure` (`/Game/Blueprints/Pickups/PickupFactories/BasePickupFactory.PickupStructure` _asbase_pickup_factory)))
  (bind _asbase_player_character (cast `/Game/Blueprints/BasePlayerCharacter` OtherActor))
  (bind _health (`/Game/Blueprints/BasePlayerCharacter.Health` _asbase_player_character))
  (bind _healthmax (`/Game/Blueprints/BasePlayerCharacter.HealthMax` _asbase_player_character))
  (if (== _health _healthmax)
    (message `/Game/Blueprints/UI/UpdateUI.SetHealth` (`/Game/Blueprints/BasePlayerController.UIReference` (cast `/Game/Blueprints/BasePlayerController` (`GameplayStatics.GetPlayerController` 0) :!pure true)) (`KismetTextLibrary.Conv_DoubleToText` _health "HalfToEven"))
    (else
      (bind _output_get (set `/Game/Blueprints/BasePlayerCharacter.Health` (`KismetMathLibrary.FClamp` (+ _health (`self.HealthToGive`)) 0.0 _healthmax) _asbase_player_character))
      (message `/Game/Blueprints/UI/UpdateUI.SetHealth` (`/Game/Blueprints/BasePlayerController.UIReference` (cast `/Game/Blueprints/BasePlayerController` (`GameplayStatics.GetPlayerController` 0) :!pure true)) (`KismetTextLibrary.Conv_DoubleToText` _output_get "HalfToEven"))
      (`/Game/Blueprints/Pickups/PickupFactories/BasePickupFactory.ReSpawn` _asbase_pickup_factory _pickupstructure_respawndelay)
      (`self.PlaySound`)
      (`self.PlayParticles`)
      (`self.K2_DestroyActor`))))

(fn `UserConstructionScript`
  (`parent.UserConstructionScript`))