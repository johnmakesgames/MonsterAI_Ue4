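; BasePickup is a base pickup actor with a configurable mesh, sound and particle effect.
; The construction script applies the custom mesh, while the SetInventory event stores an inventory reference passed in from outside.
; Both SetInventory and BeginPlay cache the first SoundManager actor found in the level.
; PlaySound routes the pickup sound through that manager, and PlayParticles spawns the emitter, both at the root component's location.
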(event `/Game/Blueprints/InventoryAllocation.SetInventory`
  (params (Inventory :type "/Game/Blueprints/Inventory Object Reference"))
  ;[1 1 1] SetupInventoryLink
  (set `self.InventoryReference` Inventory)
  (bind _outactors (`GameplayStatics.GetAllActorsOfClass` "/Game/Blueprints/SoundManager.SoundManager_C" :!label _label))
  (set `self.SoundManager` (`|GetArrayItem` _outactors)))

(event `self.ReceiveBeginPlay`
  ;[1 1 1] SetupInventoryLink
  (goto _label))

(fn `PlayParticles`
  (`GameplayStatics.SpawnEmitterAtLocation` (`self.PickupParticles`) (`SceneComponent.K2_GetComponentLocation` (`self.DefaultSceneRoot`)))
  (return))

(fn `PlaySound`
  (`/Game/Blueprints/SoundManager.PlaySFX` (`self.SoundManager`) (`self.PickUpSound`) (`SceneComponent.K2_GetComponentLocation` (`self.DefaultSceneRoot`)))
  (return))

(fn `UserConstructionScript`
  (`StaticMeshComponent.SetStaticMesh` (`self.PickupMesh`) (`self.CustomPickupMesh`)))