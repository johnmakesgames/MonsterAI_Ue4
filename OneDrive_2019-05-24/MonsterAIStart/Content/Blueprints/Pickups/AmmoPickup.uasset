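; AmmoPickup is a pickup that refills mana, bullets or missiles when a BasePlayerCharacter overlaps it.
; It branches on AmmoType and adds a clamped amount to player 0's character, rather than using the overlapping actor directly.
; It then asks its owning BasePickupFactory to respawn, plays sound and particles, updates the ammo UI if the active weapon matches, and destroys itself.
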(event `self.PickupCollision.OnComponentBeginOverlap`
  (params (OverlappedComponent :type "PrimitiveComponent Object Reference") (OtherActor :type "Actor Object Reference") (OtherComp :type "PrimitiveComponent Object Reference") (OtherBodyIndex :type Integer) (bFromSweep :type Boolean) (SweepResult :type "HitResult Structure (by ref)"))
  (bind _asbase_player_character (cast `/Game/Blueprints/BasePlayerCharacter` (`GameplayStatics.GetPlayerPawn` 0) :!pure true))
  (cast `/Game/Blueprints/BasePlayerCharacter` OtherActor)
  (switch `/Game/Blueprints/Weapons/AmmoTypes` (`self.AmmoType`)
    (:`NewEnumerator0`
      (bind _mana (`self.GiveMana` _asbase_player_character))
      (`self.UpdateUIandRespawn` _mana "/Game/Effects/FX_UsedByGregAndAde/ManaPickupGraphic.ManaPickupGraphic"))
    (:`NewEnumerator1`
      (bind _bullets (`self.GiveBullets` _asbase_player_character))
      (`self.UpdateUIandRespawn` _bullets "/Game/Effects/FX_UsedByGregAndAde/BulletPickupGraphic.BulletPickupGraphic"))
    (:`NewEnumerator2`
      (bind _missiles (`self.GiveMissiles` _asbase_player_character))
      (`self.UpdateUIandRespawn` _missiles "/Game/Effects/FX_UsedByGregAndAde/MissileGraphicPickup.MissileGraphicPickup"))))

(fn `GiveBullets`
  (params (Character :type "/Game/Blueprints/BasePlayerCharacter Object Reference"))
  (returns (Bullets :type Integer))
  (bind _output_get (set `/Game/Blueprints/BasePlayerCharacter.Bullets` (`KismetMathLibrary.Clamp` (+ (`/Game/Blueprints/BasePlayerCharacter.Bullets` Character) (`self.AmmoToGive`)) 0 (`/Game/Blueprints/BasePlayerCharacter.BulletsMax` Character)) Character))
  (return _output_get))

(fn `GiveMana`
  (params (Character :type "/Game/Blueprints/BasePlayerCharacter Object Reference"))
  (returns (Mana :type Integer))
  (bind _output_get (set `/Game/Blueprints/BasePlayerCharacter.Mana` (`KismetMathLibrary.Clamp` (+ (`/Game/Blueprints/BasePlayerCharacter.Mana` Character) (`self.AmmoToGive`)) 0 (`/Game/Blueprints/BasePlayerCharacter.ManaMax` Character)) Character))
  (return _output_get))

(fn `GiveMissiles`
  (params (Character :type "/Game/Blueprints/BasePlayerCharacter Object Reference"))
  (returns (Missiles :type Integer))
  (bind _output_get (set `/Game/Blueprints/BasePlayerCharacter.Missile` (`KismetMathLibrary.Clamp` (+ (`/Game/Blueprints/BasePlayerCharacter.Missile` Character) (`self.AmmoToGive`)) 0 (`/Game/Blueprints/BasePlayerCharacter.MissileMax` Character)) Character))
  (return _output_get))

(fn `UpdateUIandRespawn`
  (params (AmmoAmount :type Integer) (UITexture :type "Texture2D Object Reference"))
  (bind _asbase_player_controller (cast `/Game/Blueprints/BasePlayerController` (`GameplayStatics.GetPlayerController` 0) :!pure true))
  (bind _asbase_pickup_factory (cast `/Game/Blueprints/Pickups/PickupFactories/BasePickupFactory` (`self.GetOwner`) :!pure true))
  (bind (_pickupstructure_pickupclass _pickupstructure_respawndelay) (break `/Game/Blueprints/Pickups/PickupStructure` (`/Game/Blueprints/Pickups/PickupFactories/BasePickupFactory.PickupStructure` _asbase_pickup_factory)))
  ;[1 1 1] Respawn the pickup factory
  (`/Game/Blueprints/Pickups/PickupFactories/BasePickupFactory.ReSpawn` _asbase_pickup_factory _pickupstructure_respawndelay)
  (`self.PlaySound`)
  (`self.PlayParticles`)
  ;[1 1 1] If the weapon we are holding matches ammo type then update UI
  (if (`|EnumEquality` (`/Game/Blueprints/Weapons/BaseWeapon.AmmoType` (cast `/Game/Blueprints/Weapons/BaseWeapon` (`/Game/Blueprints/Inventory.ActiveWeapon` (`/Game/Blueprints/BasePlayerController.InventoryReference` _asbase_player_controller)) :!pure true)) (`self.AmmoType`))
    (`/Game/Blueprints/UI/InGameHud.SetAmmo` (`/Game/Blueprints/BasePlayerController.UIReference` _asbase_player_controller) (`KismetTextLibrary.Conv_IntToText` AmmoAmount) UITexture))
  (`self.K2_DestroyActor`)
  (return))

(fn `UserConstructionScript`
  (`parent.UserConstructionScript`))