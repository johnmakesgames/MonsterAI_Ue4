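; Base power-up pickup that the player collects into an inventory and uses for timed effects, with example logic for pickups to customize.
; Player overlap disables collision and adds non-weapon items to the inventory; a separate event plays effects, then hides or destroys the actor.
; UseItem removes depleted items from the inventory, then calls ApplyPowerUp, whose duration timer triggers RemovePowerUp.
; RemovePowerUp destroys the actor only when quantity and inventory index are both zero.
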(event `/Game/Blueprints/InventoryAllocation.SetInventory`
  (params (Inventory :type "/Game/Blueprints/Inventory Object Reference"))
  (set `self.InventoryReference` Inventory))

(event `HideorDestroy`
  (if (`self.ShouldDestroy`)
    (`self.PlaySound`)
    (`self.PlayParticles`)
    (`self.K2_DestroyActor`)
    (else
      (`self.PlaySound`)
      (`self.PlayParticles`)
      (`self.SetActorHiddenInGame` true))))

(event `self.PickupCollision.OnComponentBeginOverlap`
  (params (OverlappedComponent :type "PrimitiveComponent Object Reference") (OtherActor :type "Actor Object Reference") (OtherComp :type "PrimitiveComponent Object Reference") (OtherBodyIndex :type Integer) (bFromSweep :type Boolean) (SweepResult :type "HitResult Structure (by ref)"))
  ;[1 1 1] An Example collision logic flow, most pickups have custom event chains as they require specific functions
  (cast `/Game/Blueprints/BasePlayerCharacter` OtherActor)
  (`PrimitiveComponent.SetCollisionEnabled` (`self.PickupCollision`) "NoCollision")
  (if (not (`self.IsWeapon`))
    (`/Game/Blueprints/Inventory.AddPowerUp` (`self.InventoryReference`) self)))

(event `/Game/Blueprints/UseInventory.UseItem`
  (bind _inventoryreference (`self.InventoryReference`))
  (bind _currentitemindex (`/Game/Blueprints/Inventory.CurrentItemIndex` _inventoryreference))
  ;[1 1 1] Remove Powerup from Inventory, Apply it's Effects and then destroy the actor
  (if (== (`self.Quantity`) 0)
    (`KismetArrayLibrary.Array_RemoveItem` (`/Game/Blueprints/Inventory.Powerups` _inventoryreference) self)
    (if (== _currentitemindex 0)
      (`self.ApplyPowerUp`)
      (else
        (`/Engine/EditorBlueprintResources/StandardMacros.DecrementInt` _currentitemindex
          (:`  `
            (`self.ApplyPowerUp`)))))
    (else
      (`self.ApplyPowerUp`))))

(fn `ApplyPowerUp`
  (`KismetSystemLibrary.K2_SetTimer` self "RemovePowerUp" (`self.PowerUpDuration`))
  (return))

(fn `PlayPickupEffects`
  (return))

(fn `RemovePowerUp`
  (if (and (== (`/Game/Blueprints/Inventory.CurrentItemIndex` (`self.InventoryReference`)) 0) (== (`self.Quantity`) 0))
    (`self.K2_DestroyActor`)
    (return)
    (else
      (return))))

(fn `UserConstructionScript`
  (`parent.UserConstructionScript`))