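; Base enemy pawn that registers itself in the game mode's KillsMax total on BeginPlay and handles damage.
; AnyDamage lowers Health, then calls PlayHitEffects or PlayDeath, each spawning scaled HitFX at the BleedLocation socket and playing its sound through the game mode's SoundManager.
; PlayDeath only plays effects.
; A separate DestroyPawn, not called here, increments CurrentKills and destroys the controller and actor.
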(event `self.ReceiveBeginPlay`
  ;[1 1 1] On Intialise add to the game mode enemies stat
  (bind _output_get (set `self.GameModeRef` (cast `/Game/Blueprints/BaseGameMode` (`GameplayStatics.GetGameMode`) :!pure true)))
  (`/Engine/EditorBlueprintResources/StandardMacros.IncrementInt` (`/Game/Blueprints/BaseGameMode.KillsMax` _output_get)
    (:`  `
      (set `self.SFXManager` (`/Game/Blueprints/BaseGameMode.SoundManager` (cast `/Game/Blueprints/BaseGameMode` (`GameplayStatics.GetGameMode`) :!pure true))))))

(event `self.CapsuleComponent.OnComponentBeginOverlap`
  (params (OverlappedComponent :type "PrimitiveComponent Object Reference") (OtherActor :type "Actor Object Reference") (OtherComp :type "PrimitiveComponent Object Reference") (OtherBodyIndex :type Integer) (bFromSweep :type Boolean) (SweepResult :type "HitResult Structure (by ref)")))

(event `self.ReceiveAnyDamage`
  (params (Damage :type "Float (single-precision)") (DamageType :type "DamageType Object Reference") (InstigatedBy :type "Controller Object Reference") (DamageCauser :type "Actor Object Reference"))
  ;[1 1 1] On receive damage either die or play hit fx
  (bind _output_get (set `self.Health` (- (`self.Health`) Damage)))
  (if (<= _output_get 0.0)
    (`self.PlayDeath`)
    (else
      (`self.PlayHitEffects`))))

(fn `DestroyPawn`
  ;[1 1 1] If enemy dies add to the players kill score, then destroy the ai controller and this actor
  (`/Engine/EditorBlueprintResources/StandardMacros.IncrementInt` (`/Game/Blueprints/BaseGameMode.CurrentKills` (cast `/Game/Blueprints/BaseGameMode` (`GameplayStatics.GetGameMode`) :!pure true))
    (:`  `
      (`self.K2_DestroyActor` (`self.GetController`))
      (`self.K2_DestroyActor`))))

(fn `PlayDeath`
  (bind _returnvalue (`GameplayStatics.SpawnEmitterAtLocation` (`self.HitFX`) (`SceneComponent.GetSocketLocation` (`self.Mesh`) "BleedLocation")))
  (`/Engine/EditorBlueprintResources/StandardMacros.IsValid` _returnvalue
    (:`Is Valid`
      (`SceneComponent.SetRelativeScale3D` _returnvalue (`self.BleedingScale`)))
    (:`Is Not Valid`
      _))
  (`/Game/Blueprints/SoundManager.PlaySFX` (`/Game/Blueprints/BaseGameMode.SoundManager` (cast `/Game/Blueprints/BaseGameMode` (`GameplayStatics.GetGameMode`) :!pure true)) (`self.DeathSound`) (`self.K2_GetActorLocation`))
  (return))

(fn `PlayHitEffects`
  (bind _returnvalue (`GameplayStatics.SpawnEmitterAtLocation` (`self.HitFX`) (`SceneComponent.GetSocketLocation` (`self.Mesh`) "BleedLocation")))
  (`/Engine/EditorBlueprintResources/StandardMacros.IsValid` _returnvalue
    (:`Is Valid`
      (`SceneComponent.SetRelativeScale3D` _returnvalue (`self.BleedingScale`)))
    (:`Is Not Valid`
      _))
  (`/Game/Blueprints/SoundManager.PlaySFX` (`/Game/Blueprints/BaseGameMode.SoundManager` (cast `/Game/Blueprints/BaseGameMode` (`GameplayStatics.GetGameMode`) :!pure true)) (`self.HitSound`) (`self.K2_GetActorLocation`))
  (return))

(fn `UserConstructionScript`)