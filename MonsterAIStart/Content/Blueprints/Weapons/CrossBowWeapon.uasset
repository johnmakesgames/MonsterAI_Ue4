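; Crossbow weapon Blueprint that fires three CrossbowTriProjectile actors at once from three arrow components.
; Fire is gated by CanFire and ammo, skipping ammo use when Isinfinitefiring is set, and triggers sound and animation.
; A timeline slides the loaded arrow mesh forward from its construction-cached position, then hides it.
; A delayed Reload restores the arrow's position and visibility and re-enables firing.
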(event `self.PlayFireAnimation`
  (bind _originallocation (`self.OriginalLocation`))
  (`parent.PlayFireAnimation`)
  (`SkeletalMeshComponent.PlayAnimation` (`self.WeaponMesh`) "/Game/Meshes/Weapons/DwarfBow_Fire.DwarfBow_Fire" false)
  (`|ExecutionSequence`
    (:`then_0`
      (`KismetSystemLibrary.Delay` 1.05 :!label _label)
      (`self.Reload`))
    (:`then_1`
      (bind (_direction _positionblend) (`Timeline|Timeline_0` :!via `PlayFromStart`)
        (:`Update`
          (`SceneComponent.K2_SetRelativeLocation` (`self.SM_TD_Projectile_Arrow`) (`KismetMathLibrary.VLerp` _originallocation (+ _originallocation (100.0 0.0 0.0)) _positionblend) false false))
        (:`Finished`
          (`SceneComponent.SetVisibility` (`self.SM_TD_Projectile_Arrow`) false false)
          (goto _label))))))

(event `Reload`
  (`|ExecutionSequence`
    (:`then_0`
      (`SceneComponent.K2_SetRelativeLocation` (`self.SM_TD_Projectile_Arrow`) (`self.OriginalLocation`) false false)
      (set `self.canFire` true))
    (:`then_1`
      (`SceneComponent.SetVisibility` (`self.SM_TD_Projectile_Arrow`) true false))))

(event `self.Fire`
  (bind _arrow (`self.Arrow`))
  (bind _arrow2 (`self.Arrow2`))
  (bind _arrow1 (`self.Arrow1`))
  ;[1 1 1] Calls parent fire mechanic and spawns projectile
  (set `self.isFiring` true)
  (bind _doeshaveenoughammo (`self.CheckAmmo`))
  (if (or _doeshaveenoughammo (`self.isinfinitefiring`))
    (if (`self.canFire`)
      (set `self.canFire` false)
      (`self.PlayFireSound`)
      (if (`self.isinfinitefiring`)
        (`self.PlayFireAnimation`)
        (else
          (`self.ConsumeAmmo`)
          (`self.PlayFireAnimation`)))
      (`|SpawnActorFromClass` "/Game/Blueprints/Weapons/Projectiles/CrossbowTriProjectile.CrossbowTriProjectile_C" (`KismetMathLibrary.MakeTransform` (`SceneComponent.K2_GetComponentLocation` _arrow) (`SceneComponent.K2_GetComponentRotation` _arrow)) "AlwaysSpawn" "OverrideRootScale" null null)
      (`|SpawnActorFromClass` "/Game/Blueprints/Weapons/Projectiles/CrossbowTriProjectile.CrossbowTriProjectile_C" (`KismetMathLibrary.MakeTransform` (`SceneComponent.K2_GetComponentLocation` _arrow2) (`SceneComponent.K2_GetComponentRotation` _arrow2)) "AlwaysSpawn" "OverrideRootScale" null null)
      (`|SpawnActorFromClass` "/Game/Blueprints/Weapons/Projectiles/CrossbowTriProjectile.CrossbowTriProjectile_C" (`KismetMathLibrary.MakeTransform` (`SceneComponent.K2_GetComponentLocation` _arrow1) (`SceneComponent.K2_GetComponentRotation` _arrow1)) "AlwaysSpawn" "OverrideRootScale" null null))
    (else
      (set `self.isFiring` false))))

(fn `UserConstructionScript`
  (`parent.UserConstructionScript`)
  (set `self.OriginalLocation` (`SceneComponent.RelativeLocation` (`self.SM_TD_Projectile_Arrow`))))