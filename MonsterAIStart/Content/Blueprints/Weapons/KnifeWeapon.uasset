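; Knife weapon Blueprint that deals melee damage through overlaps on its WeaponCollision component.
; While IsFiring, an overlap applies calculated damage to enemies and other actors, skipping player characters.
; Each hit disables blade collision until a short timer restores it, preventing instant kills.
; BaseEnemy's CanBeHit flag is cleared on hit and set again when overlap ends, though this graph never checks it.
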(event `self.ReceiveBeginPlay`
  ;[1 1 1] Set blade collision enable on begin play
  (`self.ToggleCollision` true))

(event `ToggleCollision`
  (params (AdjustCollision :type Boolean))
  ;[1 1 1] Turn Blade Collision on and off
  (if AdjustCollision
    (`PrimitiveComponent.SetCollisionEnabled` (`self.WeaponCollision`) "QueryAndPhysics")
    (else
      (`PrimitiveComponent.SetCollisionEnabled` (`self.WeaponCollision`) "NoCollision"))))

(event `self.WeaponCollision.OnComponentBeginOverlap`
  (params (OverlappedComponent :type "PrimitiveComponent Object Reference") (OtherActor :type "Actor Object Reference") (OtherComp :type "PrimitiveComponent Object Reference") (OtherBodyIndex :type Integer) (bFromSweep :type Boolean) (SweepResult :type "HitResult Structure (by ref)"))
  (if (`self.isFiring`)
    (bind _asbase_enemy (cast `/Game/Blueprints/Enemies/BaseEnemy` OtherActor)
      (:`then`
        (bind _damage (`self.CalculateDamage`))
        (`GameplayStatics.ApplyDamage` _asbase_enemy _damage null null "/Game/Blueprints/Weapons/DamageType.DamageType_C")
        (if (`KismetSystemLibrary.IsValid` OtherActor)
          (set `/Game/Blueprints/Enemies/BaseEnemy.CanBeHit` false _asbase_enemy)
          (`self.ToggleCollision` false :!label _label)
          (`KismetSystemLibrary.K2_SetTimerDelegate` (delegate `hammerdamagecooldown`) 1.0)))
      (:`CastFailed`
        (cast `/Game/Blueprints/BasePlayerCharacter` OtherActor
          (:`CastFailed`
            (bind _damage_2 (`self.CalculateDamage`))
            (`GameplayStatics.ApplyDamage` OtherActor _damage_2 null null "/Game/Blueprints/Weapons/DamageType.DamageType_C")
            (goto _label)))))))

(event `hammerdamagecooldown`
  ;[1 1 1] Turns collision on again after a short while prevents insta death of enemies
  (`self.ToggleCollision` true))

(event `self.WeaponCollision.OnComponentEndOverlap`
  (params (OverlappedComponent :type "PrimitiveComponent Object Reference") (OtherActor :type "Actor Object Reference") (OtherComp :type "PrimitiveComponent Object Reference") (OtherBodyIndex :type Integer))
  ;[1 1 1] Once the blade has stopped touching the enemy allow it to hit them again in the future,
  (bind _asbase_enemy (cast `/Game/Blueprints/Enemies/BaseEnemy` OtherActor))
  (set `/Game/Blueprints/Enemies/BaseEnemy.CanBeHit` true _asbase_enemy))

(fn `UserConstructionScript`
  (`parent.UserConstructionScript`))