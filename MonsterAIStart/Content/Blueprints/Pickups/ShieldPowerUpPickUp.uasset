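; Shield power-up pickup that temporarily shields the player character.
; It overrides the parent power-up's apply and remove events to set and clear IsShielded on the first player's BasePlayerCharacter.
; On apply it also plays the shield pickup sound at the pickup mesh through SoundManager, and both events then hand off to the parent logic.
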(event `self.ApplyPowerUp`
  (set `/Game/Blueprints/BasePlayerCharacter.isShielded` true (cast `/Game/Blueprints/BasePlayerCharacter` (`GameplayStatics.GetPlayerPawn` 0) :!pure true))
  (`/Game/Blueprints/SoundManager.PlaySFX` (`self.SoundManager`) "/Game/Sounds/GregSourced/Shield_pickup_Cue.Shield_pickup_Cue" (`SceneComponent.K2_GetComponentLocation` (`self.PickupMesh`)))
  (`parent.ApplyPowerUp`))

(event `self.RemovePowerUp`
  (set `/Game/Blueprints/BasePlayerCharacter.isShielded` false (cast `/Game/Blueprints/BasePlayerCharacter` (`GameplayStatics.GetPlayerPawn` 0) :!pure true))
  (`parent.RemovePowerUp`))

(fn `UserConstructionScript`
  (`parent.UserConstructionScript`))