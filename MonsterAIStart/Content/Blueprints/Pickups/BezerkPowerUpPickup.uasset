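; Berzerk power-up pickup that temporarily raises the player character's berzerk damage.
; ApplyPowerUp sets BerzerkDamage on the first player's BasePlayerCharacter and plays a pickup sound at the mesh location through SoundManager.
; RemovePowerUp resets that damage to zero, and both events then hand off to the parent pickup's logic.
; An author note flags visual effects and sounds as needed, and no visual effect is present here.
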(event `self.ApplyPowerUp`
  ;[1 1 1] add and then remove the characters berzerk damage amount, this needs visual effects and sounds
  (set `/Game/Blueprints/BasePlayerCharacter.BerzerkDamage` 4.0 (cast `/Game/Blueprints/BasePlayerCharacter` (`GameplayStatics.GetPlayerPawn` 0) :!pure true))
  (`/Game/Blueprints/SoundManager.PlaySFX` (`self.SoundManager`) "/Game/Sounds/GregSourced/Berzerk_Pickup_Cue.Berzerk_Pickup_Cue" (`SceneComponent.K2_GetComponentLocation` (`self.PickupMesh`)))
  (`parent.ApplyPowerUp`))

(event `self.RemovePowerUp`
  ;[1 1 1] add and then remove the characters berzerk damage amount, this needs visual effects and sounds
  (set `/Game/Blueprints/BasePlayerCharacter.BerzerkDamage` 0.0 (cast `/Game/Blueprints/BasePlayerCharacter` (`GameplayStatics.GetPlayerPawn` 0) :!pure true))
  (`parent.RemovePowerUp`))

(fn `UserConstructionScript`
  (`parent.UserConstructionScript`))