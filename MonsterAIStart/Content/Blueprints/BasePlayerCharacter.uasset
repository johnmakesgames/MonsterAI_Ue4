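; Base player character that handles health, armour, death and a limited-charge forward teleport, and registers with AI sight on team 2.
; Damage drains armour before overflowing into health unless shielded; looping damage-over-time can bypass both.
; Teleport traces from the camera, with a timer restoring charges; F emits a noise event.
; Init sets class stats from SaveData or defaults to Assassin, and health and armour changes update the controller's UI.
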(event `self.ReceiveBeginPlay`
  (`AIPerceptionSystem.RegisterPerceptionStimuliSource` "/Script/AIModule.AISense_Sight" self)
  (setmembers `GenericTeamId` :`StructRef` (make `GenericTeamId` 2)))

(event `self.ReceiveAnyDamage`
  (params (Damage :type "Float (single-precision)") (DamageType :type "DamageType Object Reference") (InstigatedBy :type "Controller Object Reference") (DamageCauser :type "Actor Object Reference"))
  ;[1 1 1] if the pawn is hurt use armour to begin with
  (bind _damageleftover (`self.AdjustArmour` Damage))
  (if (> _damageleftover 0.0)
    ;[1 1 1] Is the pawn invulnerable
    (if (not (`self.isShielded`))
      ;[1 1 1] Take away current health
      (bind _nohealth (`self.RemoveHealth` _damageleftover))
      (if _nohealth
        ;[1 1 1] Play hurt effects
        (`self.PlayDeathSound`)
        (`self.PlayGibs`)
        (`self.K2_DestroyActor`)
        (else
          (`self.PlayHurtSound`)
          (`self.PlayHitEffects`))))))

(event `Key|F`
  (params (Key :type "Key Structure"))
  (:`Pressed`
    (`GameplayStatics.SpawnSoundAtLocation` "/Game/Sounds/GregSourced/End_Level_Cue.End_Level_Cue" (`self.K2_GetActorLocation`) (struct) 6.0 1.0 0.0 null null)
    (`AISense_Hearing.ReportNoiseEvent` (`self.K2_GetActorLocation` self) 1.0 self 0.0 "Noise")))

(event `DOTTimer`
  ;[1 1 1] DOT Timer
  (if (`self.IgnoreArmour&Shield`)
    (bind _nohealth (`self.RemoveHealth` (`self.DamageAmount`)))
    (if _nohealth
      (`self.PlayDeathSound`)
      (`self.PlayGibs`)
      (`self.K2_DestroyActor`)
      (else
        (`self.PlayHurtSound`)
        (`self.PlayHitEffects`)))
    (else
      (`GameplayStatics.ApplyDamage` self (`self.DamageAmount`) null null (`self.CurrentDamageType`)))))

(event `DOTStart`
  (params (DamageFrequency :type "Float (double-precision)") (DamageTypeClass :type "DamageType Class Reference") (DamageAmount :type "Float (double-precision)") (`IgnoreArmour&Shield` :type Boolean))
  ;[1 1 1] DOT start / Stop
  (set `self.DamageFrequency` DamageFrequency)
  (set `self.CurrentDamageType` DamageTypeClass)
  (set `self.DamageAmount` DamageAmount)
  (set `self.IgnoreArmour&Shield` `IgnoreArmour&Shield`)
  (`KismetSystemLibrary.K2_SetTimer` null "DOTTimer" (`self.DamageFrequency`) true))

(event `DOTStop`
  ;[1 1 1] DOT start / Stop
  (`KismetSystemLibrary.K2_ClearTimer` null "DOTTimer"))

(event `InputAction|TeleportForwards`
  (params (Key :type "Key Structure"))
  (bind _returnvalue (`GameplayStatics.GetPlayerCameraManager` 0))
  (bind _returnvalue_2 (`self.K2_GetActorLocation` _returnvalue))
  (bind _returnvalue_3 (+ _returnvalue_2 (* (`self.GetActorForwardVector` _returnvalue) (`self.Teleport Distance`))))
  ;[1 1 1] Teleport the player
  (:`Pressed`
    (if (< (`self.CurrentTeleports`) (`self.MaxTeleports`))
      (bind (_outhit _returnvalue_4) (`KismetSystemLibrary.LineTraceSingleForObjects` :`Start` _returnvalue_2 :`End` _returnvalue_3 :`ObjectTypes` (`|MakeArray` "ObjectTypeQuery1" "ObjectTypeQuery2" "ObjectTypeQuery3" "ObjectTypeQuery4" "ObjectTypeQuery5" "ObjectTypeQuery6" :!type "EObjectTypeQuery Enum") :`DrawDebugType` "ForDuration"))
      (if _returnvalue_4
        (bind (_bblockinghit _binitialoverlap _time _distance _location _impactpoint) (`GameplayStatics.BreakHitResult` _outhit))
        (bind _returnvalue_5 (`self.K2_TeleportTo` _impactpoint))
        (`GameplayStatics.PlaySound2D` "/Game/Sounds/GregSourced/Teleport_Cue.Teleport_Cue" 1.0 1.0 0.0 null null)
        (if _returnvalue_5
          (`/Engine/EditorBlueprintResources/StandardMacros.IncrementInt` (`self.CurrentTeleports`) :!label _label
            (:`  `
              (if (not (`self.TeleportRechargeTimerActive`))
                (`KismetSystemLibrary.K2_SetTimer` null "RechargeTeleport" (`self.TeleportRechargeInterval`) true)))))
        (elif (not _bblockinghit)
          (bind _returnvalue_6 (`self.K2_TeleportTo` _returnvalue_3))
          (`GameplayStatics.PlaySound2D` "/Game/Sounds/GregSourced/Teleport_Cue.Teleport_Cue" 1.0 1.0 0.0 null null)
          (if _returnvalue_6
            (goto _label)))))))

(event `RechargeTeleport`
  ;[1 1 1] Teleport Recharge Timer
  (set `self.TeleportRechargeTimerActive` true)
  (if (<= (`self.CurrentTeleports`) 0)
    (`KismetSystemLibrary.K2_ClearTimer` null "RechargeTeleport" :!label _label_2)
    (set `self.TeleportRechargeTimerActive` false)
    (else
      (bind _result (`/Engine/EditorBlueprintResources/StandardMacros.DecrementInt` (`self.CurrentTeleports`))
        (:`  `
          (if (<= _result 0)
            (goto _label_2)))))))

(fn `AdjustArmour`
  (params (Damage :type "Float (double-precision)"))
  (returns (DamageLeftOver :type "Float (double-precision)"))
  (if (> (`self.Armour`) 0.0)
    (bind _output_get (set `self.Armour` (- (`self.Armour`) Damage)))
    (if (< _output_get 0.0)
      ;[1 1 1] If we have some damage left over when the last bit of armour goes apply it onto the health bar
      (set `self.DamageModifier` (`KismetMathLibrary.Abs` _output_get))
      (bind _output_get_2 (set `self.Armour` 0.0))
      (`self.UpdateArmourUI` (`KismetTextLibrary.Conv_DoubleToText` _output_get_2 "HalfToEven"))
      (return (`self.DamageModifier`))
      (else
        ;[1 1 1] If we used up all the damage apply none to the health bar
        (`self.UpdateArmourUI` (`KismetTextLibrary.Conv_DoubleToText` (`self.Armour`) "HalfToEven"))
        (return 0.0)))
    (else
      ;[1 1 1] If we have no armour, then don't modify damage
      (return Damage))))

(fn `Init`
  (bind _returnvalue (`GameplayStatics.DoesSaveGameExist` "PlayerDataSave"))
  (if _returnvalue
    (bind _returnvalue_2 (`GameplayStatics.LoadGameFromSlot` "PlayerDataSave"))
    (bind _assave_data (cast `/Game/Blueprints/SaveData` _returnvalue_2)
      (:`then`
        (`self.SetStats` (`/Game/Blueprints/SaveData.PlayerClassData` _assave_data)))
      (:`CastFailed`
        (`self.SetStats` "NewEnumerator0" :!label _label)
        (bind _returnvalue_3 (`GameplayStatics.CreateSaveGameObject` "/Game/Blueprints/SaveData.SaveData_C"))
        (`GameplayStatics.SaveGameToSlot` _returnvalue_3 "PlayerSaveData")))
    (else
      (goto _label)))
  (return))

(fn `PlayDeathSound`
  (`GameplayStatics.SpawnSoundAtLocation` (`self.DeathSound`) (`SceneComponent.K2_GetComponentLocation` (`self.CapsuleComponent`)) (struct) 1.0 1.0 0.0 null null)
  (return))

(fn `PlayGibs`
  ;[1 1 1] Currently does nothing, should spawn some fleshy chunks, needs some glorious meshes
  (return))

(fn `PlayHitEffects`
  (`GameplayStatics.SpawnEmitterAtLocation` (`self.HitEffects`) (`SceneComponent.K2_GetComponentLocation` (`self.CapsuleComponent`)))
  (return))

(fn `PlayHurtSound`
  (`GameplayStatics.SpawnSoundAtLocation` (`self.HurtSound`) (`SceneComponent.K2_GetComponentLocation` (`self.CapsuleComponent`)) (struct) 1.0 1.0 0.0 null null)
  (return))

(fn `RemoveHealth`
  (params (Amount :type "Float (double-precision)"))
  (returns (NoHealth :type Boolean))
  (bind _output_get (set `self.Health` (- (`self.Health`) Amount)))
  (`self.UpdateHealthUI` (`KismetTextLibrary.Conv_DoubleToText` _output_get "HalfToEven"))
  (return (<= _output_get 0.0)))

(fn `SetStats`
  (params (PlayerClassData :type "/Game/Blueprints/PlayerClassType Enum" :default "NewEnumerator0"))
  (switch `/Game/Blueprints/PlayerClassType` PlayerClassData
    (:`NewEnumerator0`
      (set `self.Health` 75.0)
      (set `self.HealthMax` 100.0)
      (set `self.Armour` 75.0)
      (set `self.ArmourMax` 100.0)
      (set `self.Strength` 25)
      (set `self.Mana` 100)
      (set `self.ManaMax` 100)
      (set `self.DefaultWeapon` (`self.AssassinsDefaultWeapons`)))
    (:`NewEnumerator1`
      (set `self.Health` 75.0)
      (set `self.HealthMax` 100.0)
      (set `self.Armour` 75.0)
      (set `self.ArmourMax` 100.0)
      (set `self.Strength` 25)
      (set `self.Mana` 100)
      (set `self.ManaMax` 100)
      (set `self.DefaultWeapon` (`self.HeavysDefaultWeapons`)))
    (:`NewEnumerator2`
      (set `self.Health` 75.0)
      (set `self.HealthMax` 100.0)
      (set `self.Armour` 75.0)
      (set `self.ArmourMax` 100.0)
      (set `self.Strength` 25)
      (set `self.Mana` 100)
      (set `self.ManaMax` 100)
      (set `self.DefaultWeapon` (`self.SoldiersDefaultWeapons`))))
  (return))

(fn `UpdateArmourUI`
  (params (armour :type Text))
  (message `/Game/Blueprints/UI/UpdateUI.SetArmour` (`/Game/Blueprints/BasePlayerController.UIReference` (cast `/Game/Blueprints/BasePlayerController` (`GameplayStatics.GetPlayerController` 0) :!pure true)) armour))

(fn `UpdateHealthUI`
  (params (Health :type Text))
  (message `/Game/Blueprints/UI/UpdateUI.SetHealth` (`/Game/Blueprints/BasePlayerController.UIReference` (cast `/Game/Blueprints/BasePlayerController` (`GameplayStatics.GetPlayerController` 0) :!pure true)) Health))

(fn `UserConstructionScript`)