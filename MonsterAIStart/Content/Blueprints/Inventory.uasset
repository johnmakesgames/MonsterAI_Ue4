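; Player inventory actor that holds the first-person character's weapons and stackable powerup pickups.
; Init spawns the character's default weapons; equipping attaches one to the arms socket, sets the arm anim blueprint's weapon type and updates ammo UI.
; Weapons switch by index or by cycling those sharing a number-key tag, hiding the previous one.
; Powerups stack by name, cycle left or right, and fire through the UseInventory interface.
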(event `/Game/Blueprints/UseInventory.UseWorldItem`)

(event `/Game/Blueprints/UseInventory.UseItem`
  (bind _output (`|GetArrayItem` (`self.Powerups`) (`self.CurrentItemIndex`)))
  ;[1 1 1] Make sure array is not empty, then check currect selected entry in array and then active use item in that blueprint
  (if (== (`KismetArrayLibrary.Array_LastIndex` (`self.Powerups`)) -1)
    (`self.UpdatePowerUpUI`)
    (else
      (`/Engine/EditorBlueprintResources/StandardMacros.DecrementInt` (`/Game/Blueprints/Pickups/BasePickup.Quantity` (cast `/Game/Blueprints/Pickups/BasePowerUpPickup` _output :!pure true))
        (:`  `
          (if (`KismetSystemLibrary.DoesImplementInterface` _output "/Game/Blueprints/UseInventory.UseInventory_C")
            (message `/Game/Blueprints/UseInventory.UseItem` _output)
            (`self.UpdatePowerUpUI`)))))))

(fn `AddDefaultyInventory`
  (bind _returnvalue (`GameplayStatics.GetPlayerCharacter` 0))
  ;[1 1 1] Look for characters default weapon
  (set `self.DefaultWeaponType` (`/Game/Blueprints/BasePlayerCharacter.DefaultWeapon` (cast `/Game/Blueprints/BasePlayerCharacter` (`GameplayStatics.GetPlayerPawn` 0) :!pure true)))
  ;[1 1 1] Loop through in case they have more than one
  (for (_array_element _array_index) (`self.DefaultWeaponType`)
    ;[1 1 1] Spawn the weapon, add it to the weapons array, initialise it and then euip it
    (set `self.CurrentWeaponIndex` _array_index)
    (bind _returnvalue_2 (`|SpawnActorFromClass` (select `/Game/Blueprints/Weapons/WeaponTypes` _array_element :`NewEnumerator0` "/Game/Blueprints/Weapons/HammerWeapon.HammerWeapon_C" :`NewEnumerator1` "/Game/Blueprints/Weapons/SwordWeapon.SwordWeapon_C" :`NewEnumerator2` "/Game/Blueprints/Weapons/KnifeWeapon.KnifeWeapon_C" :`NewEnumerator3` "/Game/Blueprints/Weapons/StaffWeapon.StaffWeapon_C" :`NewEnumerator4` "/Game/Blueprints/Weapons/BaseWeapon.BaseWeapon_C" :`NewEnumerator5` "/Game/Blueprints/Weapons/CrossBowWeapon.CrossBowWeapon_C" :`NewEnumerator6` "/Game/Blueprints/Weapons/LauncherWeapon.LauncherWeapon_C" :`NewEnumerator7` "/Game/Blueprints/Weapons/RifleWeapon.RifleWeapon_C" :`NewEnumerator8` "/Game/Blueprints/Weapons/DekkerWeapon.DekkerWeapon_C" :`NewEnumerator9` "/Game/Blueprints/Weapons/TwinBlastWeapon.TwinBlastWeapon_C" :!type "/Game/Blueprints/Weapons/BaseWeapon Class Reference") (`self.GetTransform` _returnvalue) "Undefined" "OverrideRootScale" _returnvalue null))
    (bind _returnvalue_3 (`KismetArrayLibrary.Array_Add` (`self.Weapons`) _returnvalue_2))
    (`/Game/Blueprints/Weapons/BaseWeapon.Init` _returnvalue_2 self))
  (set `self.CurrentWeaponType` _array_element)
  (bind _output (`|GetArrayItem` (`self.Weapons`) _returnvalue_3))
  (`self.GiveDefaultWeaponStarterAmmo` _output)
  (`self.EquipWeapon` _output))

(fn `AddPowerUp`
  (params (ItemToAdd :type "/Game/Blueprints/Pickups/BasePowerUpPickup Object Reference"))
  (`/Engine/EditorBlueprintResources/StandardMacros.IsValid` ItemToAdd
    (:`Is Valid`
      (set `self.duplicateitemindex` -1)
      (if (not (== (`KismetArrayLibrary.Array_LastIndex` (`self.Powerups`)) -1))
        (for (_array_element _array_index) (`self.Powerups`)
          (if (== (`/Game/Blueprints/Pickups/BasePickup.Name` _array_element) (`/Game/Blueprints/Pickups/BasePickup.Name` ItemToAdd))
            (set `self.duplicateitemindex` _array_index)
            (break)
            (else
              (set `self.duplicateitemindex` -1))))
        (if (== (`self.duplicateitemindex`) -1)
          _
          (else
            (`self.AddToItemStack` (`self.duplicateitemindex`))
            (set `/Game/Blueprints/Pickups/BasePowerUpPickup.ShouldDestroy` true ItemToAdd)
            (`/Game/Blueprints/Pickups/BasePowerUpPickup.HideorDestroy` ItemToAdd)
            (`self.UpdatePowerUpUI`)
            (return))))
      (bind _returnvalue (`KismetArrayLibrary.Array_Add` (`self.Powerups`) ItemToAdd))
      (set `self.CurrentItemIndex` _returnvalue)
      (set `/Game/Blueprints/Pickups/BasePowerUpPickup.ShouldDestroy` false ItemToAdd)
      (`/Game/Blueprints/Pickups/BasePowerUpPickup.HideorDestroy` ItemToAdd)
      (`self.UpdatePowerUpUI`)
      (return))
    (:`Is Not Valid`
      (return))))

(fn `AddToItemStack`
  (params (ItemStackIndex :type Integer))
  ;[1 1 1] Increase amount of powers in inventory stack by one
  (`/Engine/EditorBlueprintResources/StandardMacros.IncrementInt` (`/Game/Blueprints/Pickups/BasePickup.Quantity` (`|GetArrayItem` (`self.Powerups`) ItemStackIndex))
    (:`  `
      (return))))

(fn `AddWeapon`
  (params (WeaponToAdd :type "Actor Class Reference") (UpdateWeaponType :type "/Game/Blueprints/Weapons/WeaponTypes Enum" :default "NewEnumerator0"))
  (bind _asbase_weapon (cast `/Game/Blueprints/Weapons/BaseWeapon` (`self.ActiveWeapon`) :!pure true))
  (set `self.CurrentWeaponType` UpdateWeaponType)
  (`/Engine/EditorBlueprintResources/StandardMacros.IsValid` _asbase_weapon
    (:`Is Valid`
      (set `/Game/Blueprints/Weapons/BaseWeapon.isFiring` false _asbase_weapon)
      (set `/Game/Blueprints/FPSArmBlueprint.Fire` false (cast `/Game/Blueprints/FPSArmBlueprint` (`SkeletalMeshComponent.GetAnimInstance` (`/Game/Blueprints/BasePlayerCharacter.FpsArms` (cast `/Game/Blueprints/BasePlayerCharacter` (`GameplayStatics.GetPlayerCharacter` 0) :!pure true))) :!pure true))
      (bind _returnvalue (`|SpawnActorFromClass` WeaponToAdd (`SceneComponent.K2_GetComponentToWorld` (`self.DefaultSceneRoot`)) "Undefined" "OverrideRootScale" null null))
      (bind _asbase_weapon_2 (cast `/Game/Blueprints/Weapons/BaseWeapon` _returnvalue :!pure true))
      (`/Game/Blueprints/Weapons/BaseWeapon.Init` _asbase_weapon_2 self)
      (bind _returnvalue_2 (`KismetArrayLibrary.Array_Add` (`self.Weapons`) _returnvalue))
      (if (`KismetSystemLibrary.IsValid` (`self.ActiveWeapon`))
        (`self.UnequipWeapon`))
      (`self.EquipWeapon` (`|GetArrayItem` (`self.Weapons`) _returnvalue_2))
      (`self.GiveDefaultWeaponStarterAmmo` _asbase_weapon_2)
      (`/Engine/EditorBlueprintResources/StandardMacros.IncrementInt` (`self.CurrentWeaponIndex`)
        (:`  `
          (return))))
    (:`Is Not Valid`
      (return))))

(fn `CheckWeapon`
  (params (WeaponToAdd :type "/Game/Blueprints/Weapons/WeaponTypes Enum" :default "NewEnumerator0"))
  (returns (ShouldAddWeapon :type Boolean))
  ;[1 1 1] Check to see if  a weapon of this class exists in the inventory, based on this return a boolean of whether we should add it or not
  (bind _filteredarray (`KismetArrayLibrary.FilterArray` (`self.Weapons`) (select `/Game/Blueprints/Weapons/WeaponTypes` WeaponToAdd :`NewEnumerator0` "/Game/Blueprints/Weapons/HammerWeapon.HammerWeapon_C" :`NewEnumerator1` "/Game/Blueprints/Weapons/SwordWeapon.SwordWeapon_C" :`NewEnumerator2` "/Game/Blueprints/Weapons/KnifeWeapon.KnifeWeapon_C" :`NewEnumerator3` "/Game/Blueprints/Weapons/StaffWeapon.StaffWeapon_C" :`NewEnumerator4` "/Game/Blueprints/Weapons/BaseWeapon.BaseWeapon_C" :`NewEnumerator5` "/Game/Blueprints/Weapons/CrossBowWeapon.CrossBowWeapon_C" :`NewEnumerator6` "/Game/Blueprints/Weapons/LauncherWeapon.LauncherWeapon_C" :`NewEnumerator7` "/Game/Blueprints/Weapons/RifleWeapon.RifleWeapon_C" :`NewEnumerator8` "/Game/Blueprints/Weapons/DekkerWeapon.DekkerWeapon_C" :`NewEnumerator9` "/Game/Blueprints/Weapons/TwinBlastWeapon.TwinBlastWeapon_C" :!type "/Game/Blueprints/Weapons/BaseWeapon Class Reference")))
  (if (== (`KismetArrayLibrary.Array_Length` _filteredarray) 0)
    (return true)
    (else
      (return false))))

(fn `CycleInventoryLeft`
  (bind _currentitemindex (`self.CurrentItemIndex`))
  ;[1 1 1] If the Array Item index is not  0  take away from current value
  (if (not (== _currentitemindex 0))
    (`/Engine/EditorBlueprintResources/StandardMacros.DecrementInt` _currentitemindex
      (:`  `
        (`self.UpdatePowerUpUI`)))))

(fn `CycleInventoryRight`
  (bind _currentitemindex (`self.CurrentItemIndex`))
  ;[1 1 1] If the Array is not empty and the Item index is not at the maximum add to the current value
  (if (== (`KismetArrayLibrary.Array_LastIndex` (`self.Powerups`)) -1)
    (`self.UpdatePowerUpUI`)
    (elif (not (== _currentitemindex (- (`KismetArrayLibrary.Array_Length` (`self.Powerups`)) 1)))
      (`/Engine/EditorBlueprintResources/StandardMacros.IncrementInt` _currentitemindex
        (:`  `
          (`self.UpdatePowerUpUI`))))))

(fn `CycleWeaponDown`
  (if (> (`self.CurrentWeaponIndex`) 0)
    (`self.UnequipWeapon`)
    (bind _result (`/Engine/EditorBlueprintResources/StandardMacros.DecrementInt` (`self.CurrentWeaponIndex`))
      (:`  `
        (bind _output (`|GetArrayItem` (`self.Weapons`) _result))
        (set `self.CurrentWeaponType` (`/Game/Blueprints/Weapons/BaseWeapon.WeaponType` (cast `/Game/Blueprints/Weapons/BaseWeapon` _output :!pure true)))
        (`self.EquipWeapon` _output)
        (set `/Game/Blueprints/FPSArmBlueprint.Fire` false (cast `/Game/Blueprints/FPSArmBlueprint` (`SkeletalMeshComponent.GetAnimInstance` (`/Game/Blueprints/BasePlayerCharacter.FpsArms` (cast `/Game/Blueprints/BasePlayerCharacter` (`GameplayStatics.GetPlayerPawn` 0) :!pure true))) :!pure true))
        (return)))
    (else
      (return))))

(fn `CycleWeaponUp`
  (if (< (`self.CurrentWeaponIndex`) (- (`KismetArrayLibrary.Array_Length` (`self.Weapons`)) 1))
    (`self.UnequipWeapon`)
    (bind _result (`/Engine/EditorBlueprintResources/StandardMacros.IncrementInt` (`self.CurrentWeaponIndex`))
      (:`  `
        (bind _output (`|GetArrayItem` (`self.Weapons`) _result))
        (set `self.CurrentWeaponType` (`/Game/Blueprints/Weapons/BaseWeapon.WeaponType` (cast `/Game/Blueprints/Weapons/BaseWeapon` _output :!pure true)))
        (`self.EquipWeapon` _output)
        (set `/Game/Blueprints/FPSArmBlueprint.Fire` false (cast `/Game/Blueprints/FPSArmBlueprint` (`SkeletalMeshComponent.GetAnimInstance` (`/Game/Blueprints/BasePlayerCharacter.FpsArms` (cast `/Game/Blueprints/BasePlayerCharacter` (`GameplayStatics.GetPlayerPawn` 0) :!pure true))) :!pure true))
        (return)))
    (else
      (return))))

(fn `DestroyInventory`
  (`self.K2_DestroyActor` (`self.ActiveWeapon`))
  (`self.K2_DestroyActor`))

(fn `EquipWeapon`
  (params (WeaponToUse :type "Actor Object Reference"))
  (bind _asbase_player_character (cast `/Game/Blueprints/BasePlayerCharacter` (`GameplayStatics.GetPlayerCharacter` 0) :!pure true))
  (bind _uireference (`/Game/Blueprints/BasePlayerController.UIReference` (cast `/Game/Blueprints/BasePlayerController` (`GameplayStatics.GetPlayerController` 0) :!pure true)))
  ;[1 1 1] Attach the weapon to the player socket
  (bind _output_get (set `self.ActiveWeapon` WeaponToUse))
  (bind _asbase_weapon (cast `/Game/Blueprints/Weapons/BaseWeapon` _output_get :!pure true))
  (set `/Game/Blueprints/Weapons/BaseWeapon.isFiring` false _asbase_weapon)
  (`self.SetActorHiddenInGame` _output_get false)
  (`self.K2_AttachRootComponentTo` _asbase_weapon (`/Game/Blueprints/BasePlayerCharacter.FpsArms` (cast `/Game/Blueprints/BasePlayerCharacter` (`GameplayStatics.GetPlayerCharacter` 0) :!pure true)) "WeaponPoint" "SnapToTargetIncludingScale" true)
  ;[1 1 1] Update the firing state to put the arms the correct position
  (bind _asbase_player_character_2 (cast `/Game/Blueprints/BasePlayerCharacter` (`GameplayStatics.GetPlayerCharacter` 0)))
  (bind _asfpsarm_blueprint (cast `/Game/Blueprints/FPSArmBlueprint` (`SkeletalMeshComponent.GetAnimInstance` (`/Game/Blueprints/BasePlayerCharacter.FpsArms` _asbase_player_character_2))))
  (bind _output_get_2 (set `self.CurrentWeaponType` (`/Game/Blueprints/Weapons/BaseWeapon.WeaponType` _asbase_weapon)))
  (set `/Game/Blueprints/FPSArmBlueprint.WeaponType` _output_get_2 _asfpsarm_blueprint)
  (`/Engine/EditorBlueprintResources/StandardMacros.IsValid` _uireference
    (:`Is Valid`
      (switch `/Game/Blueprints/Weapons/AmmoTypes` (`/Game/Blueprints/Weapons/BaseWeapon.AmmoType` (cast `/Game/Blueprints/Weapons/BaseWeapon` (`self.ActiveWeapon`) :!pure true))
        (:`NewEnumerator0`
          (`/Game/Blueprints/UI/InGameHud.SetAmmo` _uireference (`KismetTextLibrary.Conv_IntToText` (`/Game/Blueprints/BasePlayerCharacter.Mana` _asbase_player_character)) "/Game/Effects/FX_UsedByGregAndAde/ManaPickupGraphic.ManaPickupGraphic"))
        (:`NewEnumerator1`
          (`/Game/Blueprints/UI/InGameHud.SetAmmo` _uireference (`KismetTextLibrary.Conv_IntToText` (`/Game/Blueprints/BasePlayerCharacter.Bullets` _asbase_player_character)) "/Game/Effects/FX_UsedByGregAndAde/BulletPickupGraphic.BulletPickupGraphic"))
        (:`NewEnumerator2`
          (`/Game/Blueprints/UI/InGameHud.SetAmmo` _uireference (`KismetTextLibrary.Conv_IntToText` (`/Game/Blueprints/BasePlayerCharacter.Missile` _asbase_player_character)) "/Game/Effects/FX_UsedByGregAndAde/MissileGraphicPickup.MissileGraphicPickup"))
        (:`NewEnumerator3`
          (`/Game/Blueprints/UI/InGameHud.SetAmmo` _uireference "MAX" "/Game/Effects/FX_UsedByGregAndAde/MeleePickupGraphic.MeleePickupGraphic"))))))

(fn `GiveDefaultWeaponStarterAmmo`
  (params (WeaponToGiveAmmo :type "Object Object Reference"))
  (bind _asbase_player_character (cast `/Game/Blueprints/BasePlayerCharacter` (`GameplayStatics.GetPlayerCharacter` 0) :!pure true))
  (bind _asbase_player_character_2 (cast `/Game/Blueprints/BasePlayerCharacter` (`GameplayStatics.GetPlayerCharacter` 0) :!pure true))
  (bind _uireference (`/Game/Blueprints/BasePlayerController.UIReference` (cast `/Game/Blueprints/BasePlayerController` (`GameplayStatics.GetPlayerController` 0) :!pure true)))
  (switch `/Game/Blueprints/Weapons/AmmoTypes` (`/Game/Blueprints/Weapons/BaseWeapon.AmmoType` (cast `/Game/Blueprints/Weapons/BaseWeapon` WeaponToGiveAmmo :!pure true))
    (:`NewEnumerator0`
      (set `/Game/Blueprints/BasePlayerCharacter.Mana` (`KismetMathLibrary.Clamp` (+ (`/Game/Blueprints/BasePlayerCharacter.Mana` _asbase_player_character) 15) 0 (`/Game/Blueprints/BasePlayerCharacter.ManaMax` _asbase_player_character)) _asbase_player_character)
      (`/Engine/EditorBlueprintResources/StandardMacros.IsValid` _uireference
        (:`Is Valid`
          (`/Game/Blueprints/UI/InGameHud.SetAmmo` _uireference (`KismetTextLibrary.Conv_IntToText` (`/Game/Blueprints/BasePlayerCharacter.Mana` _asbase_player_character_2)) "/Game/Effects/FX_UsedByGregAndAde/ManaPickupGraphic.ManaPickupGraphic"))))
    (:`NewEnumerator1`
      (set `/Game/Blueprints/BasePlayerCharacter.Bullets` (`KismetMathLibrary.Clamp` (+ (`/Game/Blueprints/BasePlayerCharacter.Bullets` _asbase_player_character) 15) 0 (`/Game/Blueprints/BasePlayerCharacter.BulletsMax` _asbase_player_character)) _asbase_player_character)
      (`/Engine/EditorBlueprintResources/StandardMacros.IsValid` _uireference
        (:`Is Valid`
          (`/Game/Blueprints/UI/InGameHud.SetAmmo` _uireference (`KismetTextLibrary.Conv_IntToText` (`/Game/Blueprints/BasePlayerCharacter.Bullets` _asbase_player_character_2)) "/Game/Effects/FX_UsedByGregAndAde/BulletPickupGraphic.BulletPickupGraphic"))))
    (:`NewEnumerator2`
      (set `/Game/Blueprints/BasePlayerCharacter.Missile` (`KismetMathLibrary.Clamp` (+ (`/Game/Blueprints/BasePlayerCharacter.Missile` _asbase_player_character) 15) 0 (`/Game/Blueprints/BasePlayerCharacter.MissileMax` _asbase_player_character)) _asbase_player_character)
      (`/Engine/EditorBlueprintResources/StandardMacros.IsValid` _uireference
        (:`Is Valid`
          (`/Game/Blueprints/UI/InGameHud.SetAmmo` _uireference (`KismetTextLibrary.Conv_IntToText` (`/Game/Blueprints/BasePlayerCharacter.Missile` _asbase_player_character_2)) "/Game/Effects/FX_UsedByGregAndAde/MissileGraphicPickup.MissileGraphicPickup"))))
    (:`NewEnumerator3`
      (`/Engine/EditorBlueprintResources/StandardMacros.IsValid` _uireference
        (:`Is Valid`
          (`/Game/Blueprints/UI/InGameHud.SetAmmo` _uireference "MAX" "/Game/Effects/FX_UsedByGregAndAde/MeleePickupGraphic.MeleePickupGraphic")))))
  (return))

(fn `Init`
  ;[1 1 1] Setup Starting Weapons and create a reference to the owner of the inventory
  (`self.AddDefaultyInventory`)
  (`self.SetOwner` (cast `/Game/Blueprints/BasePlayerCharacter` (`GameplayStatics.GetPlayerCharacter` 0) :!pure true)))

(fn `NumberPressCycle`
  (params (WeaponTag :type Name))
  (bind _tempweapon (`self.TempWeapon`))
  (bind _output (`|GetArrayItem` (`self.TempWeapon`) (`self.TempWeaponIndex`)))
  (bind _output_2 (`|GetArrayItem` (`self.TempWeapon`)))
  ;[1 1 1] Clear Temps
  (`KismetArrayLibrary.Array_Clear` (`self.TempWeapon`))
  (set `self.TempWeaponIndex` 0)
  ;[1 1 1] Check Weapon array to see if any of them contain the tag we are pressing (this comes from player controller), if it does add them to a temp array
  (for _array_element (`self.Weapons`)
    (if (`KismetArrayLibrary.Array_Contains` (`Actor.Tags` _array_element) WeaponTag)
      (`KismetArrayLibrary.Array_Add` (`self.TempWeapon`) _array_element)))
  ;[1 1 1] Check temp array if it's empty return
  (if (> (`KismetArrayLibrary.Array_Length` (`self.TempWeapon`)) 0)
    ;[1 1 1] Check to see if current weapon is in temp array
    (if (`KismetArrayLibrary.Array_Contains` _tempweapon (`self.ActiveWeapon`))
      ;[1 1 1] Find place of current weapon in array, see if array place + 1 is larger than array length if not go to next weapon
      (bind _output_get (set `self.TempWeaponIndex` (`KismetArrayLibrary.Array_Find` _tempweapon (`self.ActiveWeapon`))))
      (if (< (- (`KismetArrayLibrary.Array_Length` (`self.TempWeapon`)) 1) (+ _output_get 1))
        ;[1 1 1] Go back to first weapon in array
        (`self.UnequipWeapon`)
        (set `self.CurrentWeaponType` (`/Game/Blueprints/Weapons/BaseWeapon.WeaponType` (cast `/Game/Blueprints/Weapons/BaseWeapon` _output_2 :!pure true)))
        (`self.EquipWeapon` _output_2)
        (set `/Game/Blueprints/FPSArmBlueprint.Fire` false (cast `/Game/Blueprints/FPSArmBlueprint` (`SkeletalMeshComponent.GetAnimInstance` (`/Game/Blueprints/BasePlayerCharacter.FpsArms` (cast `/Game/Blueprints/BasePlayerCharacter` (`GameplayStatics.GetPlayerPawn` 0) :!pure true))) :!pure true))
        (return)
        (else
          ;[1 1 1] Go to next weapon in array
          (bind _result (`/Engine/EditorBlueprintResources/StandardMacros.IncrementInt` (`self.TempWeaponIndex`))
            (:`  `
              (`self.UnequipWeapon`)
              (bind _output_3 (`|GetArrayItem` (`self.TempWeapon`) _result))
              (set `self.CurrentWeaponType` (`/Game/Blueprints/Weapons/BaseWeapon.WeaponType` (cast `/Game/Blueprints/Weapons/BaseWeapon` _output_3 :!pure true)))
              (`self.EquipWeapon` _output_3)
              (set `/Game/Blueprints/FPSArmBlueprint.Fire` false (cast `/Game/Blueprints/FPSArmBlueprint` (`SkeletalMeshComponent.GetAnimInstance` (`/Game/Blueprints/BasePlayerCharacter.FpsArms` (cast `/Game/Blueprints/BasePlayerCharacter` (`GameplayStatics.GetPlayerPawn` 0) :!pure true))) :!pure true))
              (return)))))
      (else
        ;[1 1 1] Swap to available weapon in array
        (`self.UnequipWeapon`)
        (set `self.CurrentWeaponType` (`/Game/Blueprints/Weapons/BaseWeapon.WeaponType` (cast `/Game/Blueprints/Weapons/BaseWeapon` _output :!pure true)))
        (`self.EquipWeapon` _output)
        (set `/Game/Blueprints/FPSArmBlueprint.Fire` false (cast `/Game/Blueprints/FPSArmBlueprint` (`SkeletalMeshComponent.GetAnimInstance` (`/Game/Blueprints/BasePlayerCharacter.FpsArms` (cast `/Game/Blueprints/BasePlayerCharacter` (`GameplayStatics.GetPlayerPawn` 0) :!pure true))) :!pure true))
        (return)))
    (else
      (return))))

(fn `UnequipWeapon`
  (bind _activeweapon (`self.ActiveWeapon`))
  ;[1 1 1] There are no animations currently for hiding / unequipping weapons just this toggle
  (`self.SetActorHiddenInGame` _activeweapon true)
  (`/Game/Blueprints/Weapons/BaseWeapon.StopFireAnim` (cast `/Game/Blueprints/Weapons/BaseWeapon` _activeweapon :!pure true))
  (return))

(fn `UpdatePowerUpUI`
  (bind _output (`|GetArrayItem` (`self.Powerups`) (`self.CurrentItemIndex`)))
  (bind _uireference (`/Game/Blueprints/BasePlayerController.UIReference` (cast `/Game/Blueprints/BasePlayerController` (`GameplayStatics.GetPlayerController` 0) :!pure true)))
  (if (== _output null)
    (`/Game/Blueprints/UI/InGameHud.SetPowerups` _uireference "/Game/Textures/UI/EmptyUISlot.EmptyUISlot" "")
    (else
      (`/Game/Blueprints/UI/InGameHud.SetPowerups` _uireference (`/Game/Blueprints/Pickups/BasePickup.UITexture` _output) (`KismetTextLibrary.Conv_IntToText` (`/Game/Blueprints/Pickups/BasePickup.Quantity` _output))))))

(fn `UsePowerUpEffects`)

(fn `UserConstructionScript`)