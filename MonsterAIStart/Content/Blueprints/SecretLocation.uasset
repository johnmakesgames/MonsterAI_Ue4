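; SecretLocation is a trigger actor that marks a hidden area for the player to discover.
; When a BasePlayerCharacter overlaps its Box component, it increments CurrentSecrets on the BaseGameMode.
; It then plays SecretSound at its own location and destroys itself, so each secret counts only once.
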(event `self.Box.OnComponentBeginOverlap`
  (params (OtherActor :type "Actor Object Reference") (OtherComp :type "PrimitiveComponent Object Reference") (OtherBodyIndex :type Integer) (bFromSweep :type Boolean) (SweepResult :type "HitResult Structure (by ref)"))
  ;[1 1 1] when the player enters this space addone to the current secrets found
  (cast `/Game/Blueprints/BasePlayerCharacter` OtherActor)
  (`/Engine/EditorBlueprintResources/StandardMacros.IncrementInt` (`/Game/Blueprints/BaseGameMode.CurrentSecrets` (cast `/Game/Blueprints/BaseGameMode` (`GameplayStatics.GetGameMode`) :!pure true))
    (:`  `
      (`self.PlaySecretUnlockedSound`)
      (`self.K2_DestroyActor`))))

(fn `PlaySecretUnlockedSound`
  (`GameplayStatics.SpawnSoundAtLocation` (`self.SecretSound`) (`self.K2_GetActorLocation`))
  (return))

(fn `UserConstructionScript`)