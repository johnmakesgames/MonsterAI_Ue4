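; BaseGameMode is a game mode that tracks level time and the total secret count, and handles level completion.
; On BeginPlay it counts SecretLocation actors into SecretsMax, spawns and stores a SoundManager, and starts the timer.
; A looping timer bound by function name calls AddToTime each second to advance the seconds and minutes counters.
; LevelComplete clears all widgets, shows the LevelCompleteUI, pauses the game and enables the mouse cursor.
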(event `self.ReceiveBeginPlay`
  ;[1 1 1] Store all secret areas
  (bind _outactors (`GameplayStatics.GetAllActorsOfClass` "/Game/Blueprints/SecretLocation.SecretLocation_C"))
  (set `self.SecretsMax` (`KismetArrayLibrary.Array_Length` _outactors))
  (bind _returnvalue (`|SpawnActorFromClass` "/Game/Blueprints/SoundManager.SoundManager_C" (`KismetMathLibrary.MakeTransform` (0.0 0.0 0.0)) "AlwaysSpawn" "OverrideRootScale"))
  (set `self.SoundManager` _returnvalue)
  ;[1 1 1] Trigger this in Level Blueprint / Player Pawn Sequence
  (`self.StartTimer`))

(event `LevelComplete`
  ;[1 1 1] When the level is complete open the Level Complete UI to show level stats to the player
  (`WidgetLayoutLibrary.RemoveAllWidgets`)
  (bind _returnvalue (`|CreateWidget` "/Game/Blueprints/UI/LevelCompleteUI.LevelCompleteUI_C" (`GameplayStatics.GetPlayerController` 0)))
  (`UserWidget.AddToViewport` _returnvalue 0)
  (`GameplayStatics.SetGamePaused` true)
  (set `PlayerController.bShowMouseCursor` true (cast `/Game/Blueprints/BasePlayerController` (`GameplayStatics.GetPlayerController` 0) :!pure true)))

(fn `AddToTime`
  ;[1 1 1] adds time in minutes and seconds, could easily add hours maybe a bit overkill....
  (bind _result (`/Engine/EditorBlueprintResources/StandardMacros.IncrementFloat` (`self.CurrentSeconds`))
    (:`  `
      (if (== _result 60.0)
        (set `self.CurrentSeconds` 0.0)
        (`/Engine/EditorBlueprintResources/StandardMacros.IncrementFloat` (`self.CurrentMinutes`)
          (:`  `
            (return)))
        (else
          (return))))))

(fn `StartTimer`
  (`KismetSystemLibrary.K2_SetTimer` self "AddToTime" 1.0 true)
  (return))

(fn `UserConstructionScript`)