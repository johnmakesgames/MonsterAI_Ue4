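; Sound manager Blueprint that plays sound effects at world locations and 2D music, with separate volume multipliers for each.
; Music events store the latest spawned track for stopping and live volume changes, but starting a new track does not stop the previous one.
; The J and K keys switch effects volume between full and mute and print it, affecting only subsequently played sounds.
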(event `Key|J`
  (params (Key :type "Key Structure" :default "AnyKey"))
  (:`Released`
    (bind _output_get (set `self.SoundVolume` 1.0))
    (`KismetSystemLibrary.PrintString` (`KismetStringLibrary.Conv_DoubleToString` _output_get))))

(event `Key|K`
  (params (Key :type "Key Structure" :default "AnyKey"))
  (:`Released`
    (bind _output_get (set `self.SoundVolume` 0.0))
    (`KismetSystemLibrary.PrintString` (`KismetStringLibrary.Conv_DoubleToString` _output_get))))

(event `/Game/Blueprints/SoundManagerInterface.PlaySFX`
  (params (Sound :type "SoundCue Object Reference") (Location :type "Vector Structure"))
  (`GameplayStatics.PlaySoundAtLocation` Sound Location (struct) (`self.SoundVolume`)))

(event `/Game/Blueprints/SoundManagerInterface.PlayMusic`
  (params (Sound :type "SoundCue Object Reference"))
  (bind _returnvalue (`GameplayStatics.SpawnSound2D` Sound (`self.MusicVolume`)))
  (set `self.CurrentMusicTrack` _returnvalue))

(event `/Game/Blueprints/SoundManagerInterface.StopMusic`
  (`AudioComponent.Stop` (`self.CurrentMusicTrack`)))

(event `AdjustMusicVolume`
  (params (Volume :type "Float (double-precision)"))
  (bind _currentmusictrack (`self.CurrentMusicTrack`))
  (set `self.MusicVolume` Volume)
  (`/Engine/EditorBlueprintResources/StandardMacros.IsValid` _currentmusictrack
    (:`Is Valid`
      (`AudioComponent.SetVolumeMultiplier` _currentmusictrack (`self.MusicVolume`)))))

(fn `UserConstructionScript`)